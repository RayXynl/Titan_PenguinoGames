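; Button_BP is a base button Blueprint that shows an on-screen prompt while the player character is inside its PromptBox.
; Child Blueprints set CanPrompt to decide when prompting is allowed.
; Overlap start creates the ButtonPrompt widget and sets CanPress, and overlap end removes it and clears CanPress.
; Two paired DoOnce gates reset each other so the prompt cannot stack or be removed twice.
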(event `self.PromptBox.OnComponentBeginOverlap`
  (params (OverlappedComponent :type "PrimitiveComponent Object Reference") (OtherActor :type "Actor Object Reference") (OtherComp :type "PrimitiveComponent Object Reference") (OtherBodyIndex :type Integer) (bFromSweep :type Boolean) (SweepResult :type "HitResult Structure (by ref)"))
  (if (== OtherActor (`GameplayStatics.GetPlayerCharacter` 0))
    ;[0 0 0] CanPrompt is determined within the children, allowing different cases for prompting in each
    (if (`self.CanPrompt`)
      (`/Engine/EditorBlueprintResources/StandardMacros.DoOnce` false :!label _label
        (:`Completed`
          (bind _returnvalue (`|CreateWidget` "/Game/FirstPerson/Blueprints/UI/ButtonPrompt.ButtonPrompt_C"))
          (bind _output_get (set `self.ButtonPromptWidgetRef` _returnvalue))
          (`UserWidget.AddToViewport` _output_get 0)
          (set `self.CanPress` true)
          (goto _label_2 :!via `Reset`))))))

(event `self.PromptBox.OnComponentEndOverlap`
  (params (OverlappedComponent :type "PrimitiveComponent Object Reference") (OtherActor :type "Actor Object Reference") (OtherComp :type "PrimitiveComponent Object Reference") (OtherBodyIndex :type Integer))
  (if (== OtherActor (`GameplayStatics.GetPlayerCharacter` 0))
    (`/Engine/EditorBlueprintResources/StandardMacros.DoOnce` false :!label _label_2
      (:`Completed`
        (`Widget.RemoveFromParent` (stale `self.PromptBox.OnComponentBeginOverlap` _output_get))
        (set `self.CanPress` false)
        (goto _label :!via `Reset`)))))

(fn `UserConstructionScript`)