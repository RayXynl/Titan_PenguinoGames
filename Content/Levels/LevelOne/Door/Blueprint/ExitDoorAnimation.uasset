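; Exit door Blueprint for Level One that unlocks when the game mode signals level ending, then slides open and fades the screen to black.
; Player- or enemy-tagged actors entering the trigger box turn both lights green and play a timeline that moves the door mesh and increases fade-widget opacity.
; On exit, the lights turn red and the timeline reverses, immediately for players and after a delay for enemies, without checking the lock.
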(event `self.ReceiveBeginPlay`
  (bind _aslevel_one_gamemode (cast `/Game/Levels/LevelOne/LevelOneGamemode` (`GameplayStatics.GetGameMode`)))
  (add `/Game/Levels/LevelOne/LevelOneGamemode.LevelEnding` _aslevel_one_gamemode (delegate `UnlockDoor`)))

(event `UnlockDoor`
  (set `self.Locked` false))

(event `self.Box.OnComponentBeginOverlap`
  (params (OverlappedComponent :type "PrimitiveComponent Object Reference") (OtherActor :type "Actor Object Reference") (OtherComp :type "PrimitiveComponent Object Reference") (OtherBodyIndex :type Integer) (bFromSweep :type Boolean) (SweepResult :type "HitResult Structure (by ref)"))
  (if (and (or (`ActorComponent.ComponentHasTag` (`Actor.RootComponent` OtherActor) "Player") (`ActorComponent.ComponentHasTag` (`Actor.RootComponent` OtherActor) "Enemy")) (not (`self.Locked`)))
    (set `self.ActorsWithin` (+ (`self.ActorsWithin`) 1))
    (`LightComponent.SetLightColor` (`self.PointLight`) (struct :`G` 1.0 :`A` 1.0) true)
    (`LightComponent.SetLightColor` (`self.PointLight1`) (struct :`G` 1.0 :`A` 1.0) true)
    (bind _returnvalue (`|CreateWidget` "/Game/Levels/EndGameState/WB_FadeToBlack.WB_FadeToBlack_C"))
    (`UserWidget.AddToViewport` _returnvalue 0)
    (bind (_direction _newtrack_0) (`Timeline|DoorSlide` :!label _label)
      (:`Update`
        (`SceneComponent.K2_SetRelativeLocation` (`self.FuturisticDoor_Seperated_polySurface37`) _newtrack_0 false false)
        (`/Game/Levels/EndGameState/WB_FadeToBlack.IncreaseOpacity` _returnvalue)))))

(event `self.Box.OnComponentEndOverlap`
  (params (OverlappedComponent :type "PrimitiveComponent Object Reference") (OtherActor :type "Actor Object Reference") (OtherComp :type "PrimitiveComponent Object Reference") (OtherBodyIndex :type Integer))
  (if (`ActorComponent.ComponentHasTag` (`Actor.RootComponent` OtherActor) "Player")
    (`LightComponent.SetLightColor` (`self.PointLight`) (struct :`R` 1.0 :`A` 1.0) true :!label _label_2)
    (`LightComponent.SetLightColor` (`self.PointLight1`) (struct :`R` 1.0 :`A` 1.0) true)
    (goto _label :!via `Reverse`)
    (elif (`ActorComponent.ComponentHasTag` (`Actor.RootComponent` OtherActor) "Enemy")
      (`KismetSystemLibrary.Delay` 5.0)
      (goto _label_2))))

(fn `UserConstructionScript`)