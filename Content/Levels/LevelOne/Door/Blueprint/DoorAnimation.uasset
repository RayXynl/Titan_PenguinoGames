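; Automatic sliding door that opens when an actor whose root component is tagged Player or Enemy enters its trigger box.
; Overlap plays the DoorSlide timeline to move the door mesh and turns two point lights green, with a delayed slam sound gated by a DoOnce.
; Exit turns the lights red and reverses the slide, immediately for players and after a delay for enemies.
; ActorsWithin counts entries but is never decremented or checked before closing.
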(event `self.Box.OnComponentBeginOverlap`
  (params (OverlappedComponent :type "PrimitiveComponent Object Reference") (OtherActor :type "Actor Object Reference") (OtherComp :type "PrimitiveComponent Object Reference") (OtherBodyIndex :type Integer) (bFromSweep :type Boolean) (SweepResult :type "HitResult Structure (by ref)"))
  (if (or (`ActorComponent.ComponentHasTag` (`Actor.RootComponent` OtherActor) "Player") (`ActorComponent.ComponentHasTag` (`Actor.RootComponent` OtherActor) "Enemy"))
    (set `self.ActorsWithin` (+ (`self.ActorsWithin`) 1))
    (`LightComponent.SetLightColor` (`self.PointLight`) (struct :`G` 1.0 :`A` 1.0) true)
    (`LightComponent.SetLightColor` (`self.PointLight1`) (struct :`G` 1.0 :`A` 1.0) true)
    (bind (_direction _newtrack_0) (`Timeline|DoorSlide` :!label _label)
      (:`Update`
        (`SceneComponent.K2_SetRelativeLocation` (`self.FuturisticDoor_Seperated_polySurface37`) _newtrack_0 false false)
        (`KismetSystemLibrary.Delay` 0.5)
        ;[1 1 1] audio for the door opening and closing (currently not the best, it'll loop audio for every open and close)
        (`/Engine/EditorBlueprintResources/StandardMacros.DoOnce` false :!label _label_2
          (:`Completed`
            (`GameplayStatics.PlaySoundAtLocation` "/Game/Sound/Door_Sounds/Door_Slam.Door_Slam" (`SceneComponent.K2_GetComponentLocation` (`self.DefaultSceneRoot`)) (struct) 0.5 1.0 0.0 "/Game/AudioFiles/PlaysAtLocation.PlaysAtLocation" null null null))))
      (:`Finished`
        (goto _label_2 :!via `Reset`)))))

(event `self.Box.OnComponentEndOverlap`
  (params (OverlappedComponent :type "PrimitiveComponent Object Reference") (OtherActor :type "Actor Object Reference") (OtherComp :type "PrimitiveComponent Object Reference") (OtherBodyIndex :type Integer))
  (if (`ActorComponent.ComponentHasTag` (`Actor.RootComponent` OtherActor) "Player")
    (`LightComponent.SetLightColor` (`self.PointLight`) (struct :`R` 1.0 :`A` 1.0) true :!label _label_3)
    (`LightComponent.SetLightColor` (`self.PointLight1`) (struct :`R` 1.0 :`A` 1.0) true)
    (goto _label :!via `Reverse`)
    (elif (`ActorComponent.ComponentHasTag` (`Actor.RootComponent` OtherActor) "Enemy")
      (`KismetSystemLibrary.Delay` 5.0)
      (goto _label_3))))

(fn `UserConstructionScript`)