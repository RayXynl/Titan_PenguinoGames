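; BombButton_BP is a LevelOne button actor that flags when the player can be prompted to interact with it.
; Overlapping BeginBox with the player character sets CanPrompt, but only if LevelOneGamemode is neither timing nor malfunctioning.
; Leaving the box clears the flag; this graph only sets CanPrompt and does not display the prompt or handle the press.
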(event `self.BeginBox.OnComponentBeginOverlap`
  (params (OverlappedComponent :type "PrimitiveComponent Object Reference") (OtherActor :type "Actor Object Reference") (OtherComp :type "PrimitiveComponent Object Reference") (OtherBodyIndex :type Integer) (bFromSweep :type Boolean) (SweepResult :type "HitResult Structure (by ref)"))
  (if (== OtherActor (`GameplayStatics.GetPlayerCharacter` 0))
    ;[0 0 0] Can only prompt when timer is NOT running AND is NOT malfunctioning.
    (bind _aslevel_one_gamemode (cast `/Game/Levels/LevelOne/LevelOneGamemode` (`GameplayStatics.GetGameMode`)))
    (if (`/Game/Levels/LevelOne/LevelOneGamemode.isTiming` _aslevel_one_gamemode)
      _
      (elif (not (`/Game/Levels/LevelOne/LevelOneGamemode.isMalfunctioning` _aslevel_one_gamemode))
        (set `self.CanPrompt` true)))))

(event `self.BeginBox.OnComponentEndOverlap`
  (params (OverlappedComponent :type "PrimitiveComponent Object Reference") (OtherActor :type "Actor Object Reference") (OtherComp :type "PrimitiveComponent Object Reference") (OtherBodyIndex :type Integer))
  (if (== OtherActor (`GameplayStatics.GetPlayerCharacter` 0))
    (set `self.CanPrompt` false)))

(fn `UserConstructionScript`
  (`parent.UserConstructionScript`))