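; GeneratorButton_BP is a Level One generator button that plays looping generator ambience and tracks whether the player can be prompted at it.
; BeginPlay replays the sound at the world origin through a self-looping Delay.
; Player overlap with ResumeBox sets CanPrompt only while LevelOneGamemode is malfunctioning and not timing, and leaving clears it.
; Nothing in these graphs reads CanPrompt.
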(event `self.ReceiveBeginPlay`
  ;[0 1 0.2292] referenced audio
  (`GameplayStatics.PlaySoundAtLocation` "/Game/AudioFiles/generator_ambience.generator_ambience" (0.0 0.0 0.0) (struct) 1.0 1.0 0.0 "/Game/AudioFiles/PlaysAtLocation.PlaysAtLocation" null null null :!label _label)
  (`KismetSystemLibrary.Delay` 16.77)
  (goto _label))

(event `self.ResumeBox.OnComponentBeginOverlap`
  (params (OverlappedComponent :type "PrimitiveComponent Object Reference") (OtherActor :type "Actor Object Reference") (OtherComp :type "PrimitiveComponent Object Reference") (OtherBodyIndex :type Integer) (bFromSweep :type Boolean) (SweepResult :type "HitResult Structure (by ref)"))
  (if (== OtherActor (`GameplayStatics.GetPlayerCharacter` 0))
    ;[0 0 0] Can only prompt when timer is NOT running and IS malfunctioning
    (bind _aslevel_one_gamemode (cast `/Game/Levels/LevelOne/LevelOneGamemode` (`GameplayStatics.GetGameMode`)))
    (if (`/Game/Levels/LevelOne/LevelOneGamemode.isTiming` _aslevel_one_gamemode)
      _
      (elif (`/Game/Levels/LevelOne/LevelOneGamemode.isMalfunctioning` _aslevel_one_gamemode)
        (set `self.CanPrompt` true)))))

(event `self.ResumeBox.OnComponentEndOverlap`
  (params (OverlappedComponent :type "PrimitiveComponent Object Reference") (OtherActor :type "Actor Object Reference") (OtherComp :type "PrimitiveComponent Object Reference") (OtherBodyIndex :type Integer))
  (if (== OtherActor (`GameplayStatics.GetPlayerCharacter` 0))
    (set `self.CanPrompt` false)))

(fn `UserConstructionScript`
  (`parent.UserConstructionScript`))